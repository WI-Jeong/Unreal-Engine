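; BP_Practice2 is a practice actor for per-frame movement and rotation of an actor and its components.
; Tick runs a Sequence that slides the whole actor along world X, rolls the Ch component and yaws the Ild component.
; Both components also shift relatively, Ch along Y and Ild along Z, scaled by Dir2 and Dir.
; Delta seconds scale every step for frame-rate independence, and the graph never changes either direction variable.
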(event EventBeginPlay)

(event Collision|EventActorBeginOverlap
  (params (OtherActor :type Actor%20Object%20Reference)))

(event EventTick
  (params (DeltaSeconds :type Float%20%28single-precision%29))
  (Utilities|FlowControl|Sequence
    (:then_0
      (Transformation|SetActorLocation (+ (Transformation|GetActorLocation) (Math|Vector|MakeVector (* DeltaSeconds 1.5e+02) 0.0 0.0)) false false))
    (:then_1
      ;[1 1 1] Rotation
      (Transformation|AddRelativeRotation (Variables|Default|Getch) (Math|Rotator|MakeRotator (* (Utilities|Time|GetWorldDeltaSeconds) 1.5e+02) 0.0 0.0) false false))
    (:then_2
      (Transformation|AddRelativeRotation (Variables|Default|Getild) (Math|Rotator|MakeRotator 0.0 0.0 (* (Utilities|Time|GetWorldDeltaSeconds) 1.5e+02)) false false))
    (:then_3
      ;[1 1 1] Scene component move
      (Transformation|AddRelativeLocation (Variables|Default|Getch) (Math|Vector|MakeVector 0.0 (* (Utilities|Time|GetWorldDeltaSeconds) 77.0 (Variables|Default|GetDir2)) 0.0) false false)
      (Transformation|AddRelativeLocation (Variables|Default|Getild) (Math|Vector|MakeVector 0.0 0.0 (* (Utilities|Time|GetWorldDeltaSeconds) 77.0 (Variables|Default|GetDir))) false false))))

(fn ConstructionScript)