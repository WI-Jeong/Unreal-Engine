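; BP_Practice6 is a practice actor that exercises component rotation and movement on Tick, scaled by world delta seconds.
; Each Tick yaws the Scene component, then shifts it along relative X by a speed multiplied by Dir, which this graph never changes.
; StaticMesh also gets its world location set from its relative location plus an X step, mixing coordinate spaces.
; An actor-level movement node is left disconnected.
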(event EventBeginPlay)

(event Collision|EventActorBeginOverlap
  (params (OtherActor :type Actor%20Object%20Reference)))

(event EventTick
  (params (DeltaSeconds :type Float%20%28single-precision%29))
  (Utilities|FlowControl|Sequence
    (:then_0
      (Transformation|AddRelativeRotation (Variables|Default|GetScene) (Math|Rotator|MakeRotator 0.0 0.0 (* (Utilities|Time|GetWorldDeltaSeconds) 1.5e+02)) false false))
    (:then_1
      ;[1 1 1] movement
      (Transformation|SetWorldLocation (Variables|Default|GetStaticMesh) (+ (Math|Vector|MakeVector (* (Utilities|Time|GetWorldDeltaSeconds) 1.5e+02) 0.0 0.0) (Variables|/Script/Engine.SceneComponent|GetRelativeLocation (Variables|Default|GetStaticMesh))) false false))
    (:then_2
      (Transformation|AddRelativeLocation (Variables|Default|GetScene) (Math|Vector|MakeVector (* (Utilities|Time|GetWorldDeltaSeconds) 5e+01 (Variables|Default|Getdir)) 0.0 0.0) false false))))

(fn ConstructionScript)