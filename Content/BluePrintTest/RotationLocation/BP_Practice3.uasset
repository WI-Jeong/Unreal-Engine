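; BP_Practice3 is a practice actor that spins and bobs its Scene component while moving the actor steadily along world X.
; Tick runs a Sequence that applies delta-time-scaled yaw, X movement and relative Z movement, the last signed by Dir.
; Dir flips whenever the relative Z reaches LimitDistance or drops to zero or below.
; An unconnected time-based direction flip using LimitTime remains in the graph but never runs.
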(event EventBeginPlay)

(event Collision|EventActorBeginOverlap
  (params (OtherActor :type Actor%20Object%20Reference)))

(event EventTick
  (params (DeltaSeconds :type Float%20%28single-precision%29))
  (Utilities|FlowControl|Sequence
    (:then_0
      ;[1 1 1] Rotation
      (Transformation|AddRelativeRotation (Variables|Default|GetScene) (Math|Rotator|MakeRotator 0.0 0.0 (* DeltaSeconds 1.5e+02)) false false))
    (:then_1
      (Transformation|SetActorLocation (+ (Transformation|GetActorLocation) (Math|Vector|MakeVector (* (Utilities|Time|GetWorldDeltaSeconds) 1.5e+02) 0.0 0.0)) false false))
    (:then_2
      ;[1 1 1] Go up and down by time
      (Transformation|AddRelativeLocation (Variables|Default|GetScene) (Math|Vector|MakeVector 0.0 0.0 (* (Utilities|Time|GetWorldDeltaSeconds) 3e+01 (Variables|Default|Getdir))) false false))
    (:then_3
      ;[1 1 1] 방향전환 거리
      (if (>= (.Z (Math|Vector|BreakVector (Variables|/Script/Engine.SceneComponent|GetRelativeLocation (Variables|Default|GetScene)))) (Variables|Default|Getlimit%20distance))
        (Variables|Default|Setdir (* (Variables|Default|Getdir) -1.0) :!label _label)
        (elif (<= (.Z (Math|Vector|BreakVector (Variables|/Script/Engine.SceneComponent|GetRelativeLocation (Variables|Default|GetScene)))) 0.0)
          (goto _label))))))

(fn ConstructionScript)