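; BP_Practice9 is a practice Blueprint that animates its components' rotation and location every Tick using delta-time scaling.
; A Sequence spins the Scene component in yaw and moves it along relative Z, signed by Dir, which this graph never changes.
; It also moves SkeletalMesh along X by passing its relative location plus an offset to SetWorldLocation, mixing coordinate spaces.
; An actor-level SetActorLocation move is left unconnected.
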(event EventBeginPlay)

(event Collision|EventActorBeginOverlap
  (params (OtherActor :type Actor%20Object%20Reference)))

(event EventTick
  (params (DeltaSeconds :type Float%20%28single-precision%29))
  (Utilities|FlowControl|Sequence
    (:then_0
      (Transformation|AddRelativeRotation (Variables|Default|GetScene) (Math|Rotator|MakeRotator 0.0 0.0 (* 1.5e+02 (Utilities|Time|GetWorldDeltaSeconds))) false false))
    (:then_1
      ;[1 1 1] MoveFwd
      (Transformation|SetWorldLocation (Variables|Default|GetSkeletalMesh) (+ (Math|Vector|MakeVector (* (Utilities|Time|GetWorldDeltaSeconds) 5e+01) 0.0 0.0) (Variables|/Script/Engine.SceneComponent|GetRelativeLocation (Variables|Default|GetSkeletalMesh))) false false))
    (:then_2
      (Transformation|AddRelativeLocation (Variables|Default|GetScene) (Math|Vector|MakeVector 0.0 0.0 (* 5e+01 (Utilities|Time|GetWorldDeltaSeconds) (Variables|Default|Getdir))) false false))))

(fn ConstructionScript)