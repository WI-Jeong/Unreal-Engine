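; BP_Practice8 is a practice actor that spins its static mesh while travelling along the world X axis.
; Each Tick, a Sequence first adds relative yaw to the StaticMesh, then offsets the actor location without sweeping.
; Both steps scale fixed speeds by world delta seconds, keeping the motion frame-rate independent.
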(event EventBeginPlay)

(event Collision|EventActorBeginOverlap
  (params (OtherActor :type Actor%20Object%20Reference)))

(event EventTick
  (params (DeltaSeconds :type Float%20%28single-precision%29))
  (Utilities|FlowControl|Sequence
    (:then_0
      (Transformation|AddRelativeRotation (Variables|Default|GetStaticMesh) (Math|Rotator|MakeRotator 0.0 0.0 (* (Utilities|Time|GetWorldDeltaSeconds) 7e+02)) false false))
    (:then_1
      (Transformation|SetActorLocation (+ (Transformation|GetActorLocation) (Math|Vector|MakeVector (* (Utilities|Time|GetWorldDeltaSeconds) 3e+02) 0.0 0.0)) false false))))

(fn ConstructionScript)