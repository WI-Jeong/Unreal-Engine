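; BP_Practice7 is a practice actor for rotation and location that spins and moves continuously.
; Each Tick, a Sequence first adds a relative yaw rotation to the Scene component, then moves the actor along world X without sweeping.
; Both steps scale a constant rate by world delta seconds, so the motion is frame-rate independent.
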(event EventBeginPlay)

(event Collision|EventActorBeginOverlap
  (params (OtherActor :type Actor%20Object%20Reference)))

(event EventTick
  (params (DeltaSeconds :type Float%20%28single-precision%29))
  (Utilities|FlowControl|Sequence
    (:then_0
      (Transformation|AddRelativeRotation (Variables|Default|GetScene) (Math|Rotator|MakeRotator 0.0 0.0 (* 1.5e+02 (Utilities|Time|GetWorldDeltaSeconds))) false false))
    (:then_1
      (Transformation|SetActorLocation (+ (Transformation|GetActorLocation) (Math|Vector|MakeVector (* 1.5e+02 (Utilities|Time|GetWorldDeltaSeconds)) 0.0 0.0)) false false))))

(fn ConstructionScript)